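; Demo-room display actor that shows the classic UMG settings menu on a widget component, opened to a chosen tab.
; On BeginPlay, after a short delay to dodge a visual race condition, it forces the menu container visible and switches to the tab picked by WidgetDisplay, without click animation.
; The construction script attempts the same tab switch for editor preview, which its comment notes does not work.
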(event EventBeginPlay
  (bind _widgetdisplay (Variables|Default|GetWidgetDisplay))
  (Utilities|FlowControl|Delay 0.05) ; Fix Visual Race condition in this example
  (bind _aswb_classic_settings_main (Utilities|Casting|CastToWB_ClassicSettingsMain (UserInterface|GetUserWidgetObject (Variables|Default|GetWidget))))
  (Widget|SetVisibility (Variables|/Game/QualityMenu/HUD_UMG_Classic/WB_ClassicSettingsMain.WB_ClassicSettingsMain_C|GetVerticalBox%20Main%20Container _aswb_classic_settings_main) "HitTestInvisible") ; Force menu to be displayed
  (Default|SwitchTab _aswb_classic_settings_main (Utilities|Select :Index _widgetdisplay :Option%200 (Variables|/Game/QualityMenu/HUD_UMG_Classic/WB_ClassicSettingsMain.WB_ClassicSettingsMain_C|GetTab%20Audio%20Settings _aswb_classic_settings_main) :Option%201 (Variables|/Game/QualityMenu/HUD_UMG_Classic/WB_ClassicSettingsMain.WB_ClassicSettingsMain_C|GetTab%20Video%20Settings _aswb_classic_settings_main) :Option%202 (Variables|/Game/QualityMenu/HUD_UMG_Classic/WB_ClassicSettingsMain.WB_ClassicSettingsMain_C|GetTabCameraSettings _aswb_classic_settings_main) :Option%203 (Variables|/Game/QualityMenu/HUD_UMG_Classic/WB_ClassicSettingsMain.WB_ClassicSettingsMain_C|GetTabKeySettings _aswb_classic_settings_main) :Option%204 (Variables|/Game/QualityMenu/HUD_UMG_Classic/WB_ClassicSettingsMain.WB_ClassicSettingsMain_C|GetTab%20Game%20Settings _aswb_classic_settings_main) :Option%205 (Variables|/Game/QualityMenu/HUD_UMG_Classic/WB_ClassicSettingsMain.WB_ClassicSettingsMain_C|GetTabDevelopmentSettings _aswb_classic_settings_main)) _widgetdisplay false))

(fn ConstructionScript
  (bind _widgetdisplay (Variables|Default|GetWidgetDisplay))
  ;[1 1 1] This does not work in editor D:
  (bind _aswb_classic_settings_main (Utilities|Casting|CastToWB_ClassicSettingsMain (UserInterface|GetUserWidgetObject (Variables|Default|GetWidget))))
  (Default|SwitchTab _aswb_classic_settings_main (Utilities|Select :Index _widgetdisplay :Option%200 (Variables|/Game/QualityMenu/HUD_UMG_Classic/WB_ClassicSettingsMain.WB_ClassicSettingsMain_C|GetTab%20Audio%20Settings _aswb_classic_settings_main) :Option%201 (Variables|/Game/QualityMenu/HUD_UMG_Classic/WB_ClassicSettingsMain.WB_ClassicSettingsMain_C|GetTab%20Video%20Settings _aswb_classic_settings_main) :Option%202 (Variables|/Game/QualityMenu/HUD_UMG_Classic/WB_ClassicSettingsMain.WB_ClassicSettingsMain_C|GetTabCameraSettings _aswb_classic_settings_main) :Option%203 (Variables|/Game/QualityMenu/HUD_UMG_Classic/WB_ClassicSettingsMain.WB_ClassicSettingsMain_C|GetTabKeySettings _aswb_classic_settings_main) :Option%204 (Variables|/Game/QualityMenu/HUD_UMG_Classic/WB_ClassicSettingsMain.WB_ClassicSettingsMain_C|GetTab%20Game%20Settings _aswb_classic_settings_main) :Option%205 (Variables|/Game/QualityMenu/HUD_UMG_Classic/WB_ClassicSettingsMain.WB_ClassicSettingsMain_C|GetTabDevelopmentSettings _aswb_classic_settings_main)) _widgetdisplay false))