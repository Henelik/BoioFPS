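; Demo display Blueprint that shows several input key bindings in one TextRender, each wrapped in its configured pre and post text.
; At BeginPlay it resolves each mapping's combination from GameSettings and rebuilds the text whenever one updates.
; The construction script creates dummy combinations from DT_InputActionList for editor preview.
; Unresolved entries keep their array slot and display placeholder text, with invalid names also printed at runtime.
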(event Custom|Combination%20Updated
  (params (Combination :type BP%20Key%20Combination%20Object%20Reference))
  (Variables|Default|SetDisplay%20Text "")
  (for (_array_element _array_index) (Variables|Default|GetMappings)
    (Utilities|IsValid (Utilities|Array|Get(acopy) (Variables|Default|GetCombinations) _array_index)
      (:Is%20Valid
        (bind _display_name (Default|GetKeyCombinationDisplayName (Utilities|Array|Get(acopy) (Variables|Default|GetCombinations) _array_index) " + " "None" "NewEnumerator1"))
        (Variables|Default|SetDisplay%20Text (Utilities|String|Append (Variables|Default|GetDisplay%20Text) (Utilities|String|Append (.pretext _array_element) _display_name (.posttext _array_element)))))
      (:Is%20Not%20Valid
        (Variables|Default|SetDisplay%20Text (Utilities|String|Append (Variables|Default|GetDisplay%20Text) (Utilities|String|Append (.pretext _array_element) (select (or (Utilities|Enum|Equal(Enum) (.actionname _array_element) "") (Utilities|Enum|Equal(Enum) (.mappingname _array_element) "")) "#Input#" "#ERRORKEY#") (.posttext _array_element)))) ; Key Missing
      )))
  (|UpdateTextRender))

(event EventBeginPlay
  (bind _game_settings (Utilities|GetGameSettings (Game|GetGameInstance)))
  (Variables|Default|SetGame%20Settings _game_settings)
  (Utilities|Array|Clear (Variables|Default|GetCombinations))
  (for _array_element (Variables|Default|GetMappings)
    (bind (_combination _success) (Utilities|GetKeyCombination (Variables|Default|GetGame%20Settings) (.actionname _array_element) (.mappingname _array_element) (.secondarymapping _array_element)))
    (if _success
      (Utilities|Array|Add (Variables|Default|GetCombinations) _combination)
      (EventDispatchers|AssignCombinationUpdated _combination (delegate Custom|Combination%20Updated))
      (else
        (Development|PrintString (Utilities|String|Append "Invalid action or mapping name in " (Utilities|GetDisplayName self) "."))
        (Utilities|Array|Add (Variables|Default|GetCombinations) 0) ; Add Empty Object on to array to keep length\nconsistent with Mappings Array
      )))
  (Variables|Default|SetDisplay%20Text "")
  (for (_array_element_2 _array_index) (Variables|Default|GetMappings)
    (Utilities|IsValid (Utilities|Array|Get(acopy) (Variables|Default|GetCombinations) _array_index)
      (:Is%20Valid
        (bind _display_name (Default|GetKeyCombinationDisplayName (Utilities|Array|Get(acopy) (Variables|Default|GetCombinations) _array_index) " + " "None" "NewEnumerator1"))
        (Variables|Default|SetDisplay%20Text (Utilities|String|Append (Variables|Default|GetDisplay%20Text) (Utilities|String|Append (.pretext _array_element_2) _display_name (.posttext _array_element_2)))))
      (:Is%20Not%20Valid
        (Variables|Default|SetDisplay%20Text (Utilities|String|Append (Variables|Default|GetDisplay%20Text) (Utilities|String|Append (.pretext _array_element_2) (select (or (Utilities|Enum|Equal(Enum) (.actionname _array_element_2) "") (Utilities|Enum|Equal(Enum) (.mappingname _array_element_2) "")) "#Input#" "#ERRORKEY#") (.posttext _array_element_2)))) ; Key Missing
      )))
  (|UpdateTextRender))

(fn ConstructionScript
  (for _array_element (Variables|Default|GetMappings)
    (LocalVariables|SetAction%20Name (.actionname _array_element))
    (LocalVariables|SetMapping%20Name (.mappingname _array_element))
    (LocalVariables|SetSecondary%20Mapping (.secondarymapping _array_element))
    (LocalVariables|SetBinding%20Combination 0)
    (bind _outrownames (DataTable|GetDataTableRowNames "/Game/QualityMenu/Blueprints/DT_InputActionList.DT_InputActionList"))
    (for _array_element_2 _outrownames
      (if (Utilities|Enum|Equal(Enum) (Utilities|String|ToString(Name) _array_element_2) (LocalVariables|GetAction%20Name))
        (bind _returnvalue (Utilities|GetDataTableRow "/Game/QualityMenu/Blueprints/DT_InputActionList.DT_InputActionList" _array_element_2)
          (:then
            (for _array_element_3 (.KeyMappings (Utilities|Struct|BreakSKeyAction _returnvalue))
              (if (Utilities|Enum|Equal(Enum) (.name _array_element_3) (LocalVariables|GetMapping%20Name))
                (bind _returnvalue_2 (Game|ConstructObjectfromClass "/Game/QualityMenu/Blueprints/Util/Keybinding/BP_KeyCombination.BP_KeyCombination_C" self)) ; Create dummy combination only used in editor
                (bind _output_get (LocalVariables|SetBinding%20Combination _returnvalue_2))
                (if (LocalVariables|GetSecondary%20Mapping)
                  (Default|ReplaceKeyCombination _output_get (.secondarycombination _array_element_3))
                  (else
                    (Default|ReplaceKeyCombination _output_get (.primarycombination _array_element_3))))))))))
    (Utilities|Array|Add (Variables|Default|GetCombinations) (LocalVariables|GetBinding%20Combination)))
  (CallFunction|CombinationUpdated))