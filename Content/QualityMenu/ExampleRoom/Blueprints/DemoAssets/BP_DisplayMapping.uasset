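; BP_DisplayMapping is a demo asset that renders the key bound to a named input action mapping as text, wrapped in configurable pre/post text.
; At BeginPlay it fetches the primary or secondary combination from GameSettings and binds to its update event, keeping the text current.
; The construction script builds a dummy combination from DT_InputActionList for editor preview.
; Invalid combinations show placeholder or error text, and failed runtime lookups also print an error.
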(event Custom|Combination%20Updated
  (params (Combination :type BP%20Key%20Combination%20Object%20Reference))
  (Utilities|IsValid Combination
    (:Is%20Valid
      (bind _display_name (Default|GetKeyCombinationDisplayName Combination " + " "None" "NewEnumerator1"))
      (Rendering|Components|TextRender|SetText (Variables|Default|GetTextRender) (Utilities|Text|ToText(String) (Utilities|String|Append (Variables|Default|GetPretext) _display_name (Variables|Default|GetPosttext))))
      (Rendering|Components|TextRender|SetHorizontalAlignment (Variables|Default|GetTextRender) (Variables|Default|GetText%20Alignment)))
    (:Is%20Not%20Valid
      (Rendering|Components|TextRender|SetText (Variables|Default|GetTextRender) (Utilities|Text|ToText(String) (Utilities|String|Append (Variables|Default|GetPretext) (select (or (Utilities|Enum|Equal(Enum) (Variables|Default|GetAction%20Name) "") (Utilities|Enum|Equal(Enum) (Variables|Default|GetMapping%20Name) "")) "#Input#" "#ERRORKEY#") (Variables|Default|GetPosttext)))) ; Error text
      (Rendering|Components|TextRender|SetHorizontalAlignment (Variables|Default|GetTextRender) (Variables|Default|GetText%20Alignment)))))

(event EventBeginPlay
  (bind _game_settings (Utilities|GetGameSettings (Game|GetGameInstance)))
  (bind _output_get (Variables|Default|SetGame%20Settings _game_settings))
  (bind (_combination _success) (Utilities|GetKeyCombination _output_get (Variables|Default|GetAction%20Name) (Variables|Default|GetMapping%20Name) (Variables|Default|GetSecondary%20Mapping)))
  (if _success
    (bind _output_get_2 (Variables|Default|SetBinding%20Combination _combination))
    (EventDispatchers|AssignCombinationUpdated _output_get_2 (delegate Custom|Combination%20Updated))
    (CallFunction|CombinationUpdated _output_get_2) ; Update Combination so we don't\nwait for a change to trigger it
    (else
      (Development|PrintString (Utilities|String|Append "Err: \"" (Utilities|GetDisplayName self) "\" has incorrect action or mapping name") true true "(R=0.000000,G=0.660000,B=1.000000,A=1.000000)" 4.0)
      (Rendering|Components|TextRender|SetText (Variables|Default|GetTextRender) (Utilities|Text|ToText(String) (Utilities|String|Append (Variables|Default|GetPretext) (select (or (Utilities|Enum|Equal(Enum) (Variables|Default|GetAction%20Name) "") (Utilities|Enum|Equal(Enum) (Variables|Default|GetMapping%20Name) "")) "#Input#" "#ERRORKEY#") (Variables|Default|GetPosttext)))) ; Error text
      (Rendering|Components|TextRender|SetHorizontalAlignment (Variables|Default|GetTextRender) (Variables|Default|GetText%20Alignment)))))

(fn ConstructionScript
  (bind _outrownames (DataTable|GetDataTableRowNames "/Game/QualityMenu/Blueprints/DT_InputActionList.DT_InputActionList"))
  (for _array_element _outrownames
    (if (Utilities|Enum|Equal(Enum) (Utilities|String|ToString(Name) _array_element) (Variables|Default|GetAction%20Name))
      (bind _returnvalue (Utilities|GetDataTableRow "/Game/QualityMenu/Blueprints/DT_InputActionList.DT_InputActionList" _array_element)
        (:then
          (for _array_element_2 (.KeyMappings (Utilities|Struct|BreakSKeyAction _returnvalue))
            (if (Utilities|Enum|Equal(Enum) (.name _array_element_2) (Variables|Default|GetMapping%20Name))
              (bind _returnvalue_2 (Game|ConstructObjectfromClass "/Game/QualityMenu/Blueprints/Util/Keybinding/BP_KeyCombination.BP_KeyCombination_C" self)) ; Create dummy combination only used in editor
              (bind _output_get (Variables|Default|SetBinding%20Combination _returnvalue_2))
              (if (Variables|Default|GetSecondary%20Mapping)
                (Default|ReplaceKeyCombination _output_get (.secondarycombination _array_element_2))
                (else
                  (Default|ReplaceKeyCombination _output_get (.primarycombination _array_element_2))))))))))
  (CallFunction|CombinationUpdated (Variables|Default|GetBinding%20Combination)))