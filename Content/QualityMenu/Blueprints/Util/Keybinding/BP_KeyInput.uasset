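; Key input object for the keybinding system, wrapping one key plus an axis direction, with a readable display name and saving to game settings.
; Init remaps directional keys to axis equivalents with a negative-axis flag, which name generation converts back to mouse, stick, trigger or wheel labels.
; Analog values are cached per update for press/release edge detection.
; The base state check, marked deprecated for child overrides, divides mouse movement by world delta.
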(fn InitKeyInput
  (params (Key%20Input :type S%20Key%20Input%20Structure))
  (bind _returnvalue (Utilities|ReplaceKeyMapping Key%20Input)) ; Convert some directional\nmappings to its axis equivalent
  (bind _output_get (Variables|Default|SetKey%20Input (.Input (Utilities|Struct|BreakSKeyInput _returnvalue))))
  (Variables|Default|SetAnalog%20Use%20Negative%20Axis (.UseNegativeAxis (Utilities|Struct|BreakSKeyInput _returnvalue)))
  (Variables|Default|SetInput%20is%20Using%20Delta (or (== _output_get "MouseX") (== _output_get "MouseY")))
  (CallFunction|GenerateDisplayName)
  (return self))

(fn KeyInputCurrentState
  (params (Controller :type Player%20Controller%20Object%20Reference))
  (bind _key_input (Variables|Default|GetKey%20Input))
  (bind _key_input_2 (Variables|Default|GetKey%20Input))
  (bind _analog_use_negative_axis (Variables|Default|GetAnalog%20Use%20Negative%20Axis))
  (bind _analog_previous_axis_value (Variables|Default|GetAnalog%20Previous%20Axis%20Value))
  (bind _returnvalue (Game|Player|IsInputKeyDown Controller _key_input_2))
  (bind _returnvalue_2 (Class|PlayerController|GetInputAnalogKeyState Controller _key_input))
  (bind _returnvalue_3 (< _analog_previous_axis_value 0.1))
  (bind _returnvalue_4 (>= _analog_previous_axis_value 0.1))
  (bind _returnvalue_5 (Math|Float|Min(Float) _returnvalue_2 0.0))
  (bind _returnvalue_6 (Math|Float|Max(Float) _returnvalue_2 0.0))
  (bind _returnvalue_7 (Math|Float|Absolute(Float) _returnvalue_5))
  (bind _returnvalue_8 (Math|Float|SelectFloat _returnvalue_7 _returnvalue_6 _analog_use_negative_axis))
  (bind _returnvalue_9 (>= _returnvalue_8 0.1))
  (bind _returnvalue_10 (>= _returnvalue_8 0.1))
  (bind _returnvalue_11 (< _returnvalue_8 0.1))
  (bind _returnvalue_12 (and _returnvalue_9 _returnvalue_3))
  (bind _returnvalue_13 (and _returnvalue_11 _returnvalue_4))
  ;[1 1 1] Old Keybinding Checker. Should not be used.
  ; Child blueprints overrides this function
  (Utilities|IsValid Controller
    (:Is%20Valid
      (if (Class|KismetInputLibrary|KeyIsFloatAxis _key_input_2)
        ;[1 1 1] Analog Axis Input
        (if (Variables|Default|GetInput%20is%20Using%20Delta)
          (return (* (Math|Float|MakeLiteralFloat 0.02) (/ _returnvalue_8 (Variables|Default|GetWorld%20Delta%20Seconds))) _returnvalue_10 _returnvalue_12 _returnvalue_13) ; Mouse Axis Value
          (else
            (return _returnvalue_8 _returnvalue_10 _returnvalue_12 _returnvalue_13) ; Other analog value
          ))
        (else
          ;[1 1 1] Button Input
          (return (Math|Conversions|ToFloat(Boolean) _returnvalue) _returnvalue (Game|Player|WasInputKeyJustPressed Controller _key_input_2) (Class|PlayerController|WasInputKeyJustReleased Controller _key_input_2)))))
    (:Is%20Not%20Valid
      (Development|PrintString 0 (Utilities|String|Append "Err: BP_Keyinput, " (Utilities|String|ToString(Text) (Class|KismetInputLibrary|KeyGetDisplayName (Variables|Default|GetKey%20Input))) "Player Controller is not valid."))
      (return 0.0 false false false))))

(fn UpdateAnalogAxisValue
  (params (World%20Delta%20Seconds :type Float%20%28single-precision%29) (Player%20Controller :type Player%20Controller%20Object%20Reference))
  (bind _key_input (Variables|Default|GetKey%20Input))
  (bind _returnvalue (Class|PlayerController|GetInputAnalogKeyState Player%20Controller _key_input))
  (Variables|Default|SetWorld%20Delta%20Seconds World%20Delta%20Seconds)
  (Variables|Default|SetAnalog%20Previous%20Axis%20Value (Variables|Default|GetAnalog%20Current%20Axis%20Value))
  (Variables|Default|SetAnalog%20Current%20Axis%20Value (Math|Float|SelectFloat (Math|Float|Absolute(Float) (Math|Float|Min(Float) _returnvalue 0.0)) (Math|Float|Max(Float) _returnvalue 0.0) (Variables|Default|GetAnalog%20Use%20Negative%20Axis))))

(fn SaveKeyInput
  (params (Game%20Settings :type BP%20Game%20Settings%20Object%20Reference) (KeySave :type S%20Key%20Action%20Save%20Structure%20%28by%20ref%29))
  (bind _structout (Utilities|Struct|SetmembersinSKeyActionSave KeySave (Variables|Default|GetKey%20Input) (Variables|Default|GetAnalog%20Use%20Negative%20Axis) false))
  (Default|StoreKeyInput Game%20Settings _structout))

(fn GenerateDisplayName
  (Variables|Default|SetDisplay%20Name (Utilities|String|ToString(Text) (Class|KismetInputLibrary|KeyGetDisplayName (Variables|Default|GetKey%20Input)))) ; Default Name in case\nof no replacement
  (|FindAndConvertMouseDirection)
  (|FindAndConvertAnalogAxis))