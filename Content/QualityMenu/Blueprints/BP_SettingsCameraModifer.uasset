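; Camera modifier that applies the player's game settings for field of view and image adjustments to the camera.
; It overrides FOV and supplies full-weight post-process settings for color gamma, gain and bloom intensity, expanding scalar values into Vector4s.
; Both modify hooks lazily fetch and cache GameSettings from the Game Instance, since camera modifiers lack BeginPlay.
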(fn BlueprintModifyCamera
  (params (DeltaTime :type Float%20%28single-precision%29) (ViewLocation :type Vector) (ViewRotation :type Rotator) (FOV :type Float%20%28single-precision%29))
  (CallFunction|ValidateGameSettings) ; Makes sure game settings are valid\n(Since Camera modifer don't have Begin Play event)
  (return ViewLocation ViewRotation (Default|GetFieldOfView (Variables|Default|GetGame%20Settings))))

(fn BlueprintModifyPostProcess
  (params (DeltaTime :type Float%20%28single-precision%29))
  (bind _game_settings (Variables|Default|GetGame%20Settings))
  (CallFunction|ValidateGameSettings) ; Makes sure game settings are valid\n(Since Camera modifer don't have Begin Play event)
  (return 1.0 (Utilities|Struct|MakePostProcessSettings (Utilities|FloattoVector4 (Default|GetGammaIntensity _game_settings)) (Utilities|FloattoVector4 (Default|GetGainIntensity _game_settings)) (Default|GetBloomIntensity _game_settings))))

(fn ValidateGameSettings
  (Utilities|IsValid (Variables|Default|GetGame%20Settings)
    (:Is%20Valid
      _)
    (:Is%20Not%20Valid
      (bind _game_settings (Utilities|GetGameSettings (Game|GetGameInstance)))
      (Variables|Default|SetGame%20Settings _game_settings)))
  (return))